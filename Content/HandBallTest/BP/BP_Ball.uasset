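; Handball test ball that resolves a shot on BeginPlay from the Comp_handball flags on the TargetPoint picked by ZoneIndex.
; For a save, it passes the flags to PlayerCharacterHandBall_BP and timeline-lerps to that character's hand or foot socket.
; Goal and unsaved branches start lerps involving the target, but destroy the ball on the timeline's first update.
; BallFinish only prints; manager UI calls and other leftover chains are disconnected.
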(event OnComponentBeginOverlap(BallCollision)
  (params (OverlappedComponent :type Primitive%20Component%20Object%20Reference) (OtherActor :type Actor%20Object%20Reference) (OtherComp :type Primitive%20Component%20Object%20Reference) (OtherBodyIndex :type Integer) (bFromSweep :type Boolean) (SweepResult :type Hit%20Result%20Structure%20%28by%20ref%29))
  (Transformation|SetActorRotation (* (.rotation (Transformation|GetActorTransform)) (Math|Random|RandomFloat)))
  (Physics|SetSimulatePhysics (Variables|Default|GetBallCollision) false)
  (CallFunction|BallFinish))

(event OnComponentHit(BallCollision)
  (params (HitComponent :type Primitive%20Component%20Object%20Reference) (OtherActor :type Actor%20Object%20Reference) (OtherComp :type Primitive%20Component%20Object%20Reference) (NormalImpulse :type Vector :default "0, 0, 0") (Hit :type Hit%20Result%20Structure%20%28by%20ref%29))
  (Physics|SetSimulatePhysics (Variables|Default|GetBallCollision) true))

(event Custom|BallTracker
  (Transformation|SetWorldLocation (Variables|Default|GetBallCollision self) (Transformation|GetActorLocation) false false)
  (Development|PrintString (Utilities|String|ToString(Vector) (Transformation|GetActorLocation))))

(event Custom|Ricochet
  (Physics|AddImpulse (Variables|Default|GetBall) (Math|Vector|MakeVector (Math|Random|RandomFloat) (Math|Random|RandomFloat) (Math|Random|RandomFloat)) "None" false))

(event Collision|EventActorBeginOverlap
  (params (OtherActor :type Actor%20Object%20Reference)))

(event EventBeginPlay
  (bind _ballcollision (Variables|Default|GetBallCollision))
  (bind _ballcollision_2 (Variables|Default|GetBallCollision))
  (bind _outactors (Actor|GetAllActorsOfClass "/Script/Engine.TargetPoint"))
  (if (Variables|/Game/HandBallTest/BP/comp_handball.comp_handball_C|GetIsGoal\Out? (Actor|GetComponentbyClass (Utilities|Array|Get(acopy) _outactors (stale EventBpiHandBallPass Zone_Index)) "/Game/HandBallTest/BP/comp_handball.comp_handball_C"))
    (Development|PrintString "Голл")
    (bind _floattrack (Timeline|Timeline_1 Play)
      (:Update
        (Transformation|SetWorldLocation _ballcollision_2 (Math|Vector|Lerp(Vector) (Transformation|GetActorLocation (Utilities|Array|Get(acopy) _outactors (stale EventBpiHandBallPass Zone_Index))) (Transformation|GetActorLocation) _floattrack) false false)
        (Physics|SetSimulatePhysics _ballcollision_2 true)
        (Utilities|IsValid self
          (:Is%20Valid
            (Actor|DestroyActor)))))
    (else
      (Development|PrintString "Отбил")
      (if (Variables|/Game/HandBallTest/BP/comp_handball.comp_handball_C|GetIsRefand? (Actor|GetComponentbyClass (Utilities|Array|Get(acopy) _outactors (stale EventBpiHandBallPass Zone_Index)) "/Game/HandBallTest/BP/comp_handball.comp_handball_C"))
        (bind _outactors_2 (Actor|GetAllActorsOfClass "/Game/HandBallTest/BP/PlayerCharacterHandBall_BP.PlayerCharacterHandBall_BP_C"))
        (bind _asplayer_character_hand_ball_bp (Utilities|Casting|CastToPlayerCharacterHandBall_BP (Utilities|Array|Get(acopy) _outactors_2)))
        (Utilities|FlowControl|Sequence
          (:then_0
            (Variables|/Game/HandBallTest/BP/PlayerCharacterHandBall_BP.PlayerCharacterHandBall_BP_C|SetGoal\Out? _asplayer_character_hand_ball_bp (Variables|/Game/HandBallTest/BP/comp_handball.comp_handball_C|GetIsGoal\Out? (Actor|GetComponentbyClass (Utilities|Array|Get(acopy) _outactors (stale EventBpiHandBallPass Zone_Index)) "/Game/HandBallTest/BP/comp_handball.comp_handball_C")))
            (Variables|/Game/HandBallTest/BP/PlayerCharacterHandBall_BP.PlayerCharacterHandBall_BP_C|SetRefand? _asplayer_character_hand_ball_bp (Variables|/Game/HandBallTest/BP/comp_handball.comp_handball_C|GetIsRefand? (Actor|GetComponentbyClass (Utilities|Array|Get(acopy) _outactors (stale EventBpiHandBallPass Zone_Index)) "/Game/HandBallTest/BP/comp_handball.comp_handball_C"))))
          (:then_1
            (switch Utilities|FlowControl|Switch|SwitchonE_HandBallerBodyPoints (Variables|/Game/HandBallTest/BP/comp_handball.comp_handball_C|GetE_HandBallerBodyPoints (Actor|GetComponentbyClass (Utilities|Array|Get(acopy) _outactors (stale EventBpiHandBallPass Zone_Index)) "/Game/HandBallTest/BP/comp_handball.comp_handball_C"))
              (:NewEnumerator0
                (Variables|Default|Setsocketindex 0))
              (:NewEnumerator1
                (Variables|Default|Setsocketindex 1))
              (:NewEnumerator2
                (Variables|Default|Setsocketindex 2))
              (:NewEnumerator3
                (Variables|Default|Setsocketindex 3)))
            (Utilities|FlowControl|Delay 0.2)
            (bind _floattrack_2 (Timeline|Timeline_0 Play)
              (:Update
                (Transformation|SetActorLocation (Math|Vector|Lerp(Vector) (Transformation|GetActorLocation) (Transformation|GetSocketLocation (Variables|/Script/Engine.Character|GetMesh _asplayer_character_hand_ball_bp) (Utilities|Array|Get(acopy) (Variables|/Game/HandBallTest/BP/PlayerCharacterHandBall_BP.PlayerCharacterHandBall_BP_C|GetIn%20Socket%20Name _asplayer_character_hand_ball_bp) (Variables|Default|Getsocketindex))) _floattrack_2) false false)
                (Physics|SetSimulatePhysics (Variables|Default|GetBallCollision) true)))))
        (else
          (Development|PrintString "Не Отбил")
          (bind _floattrack_3 (Timeline|Timeline_3 Play)
            (:Update
              (Transformation|SetWorldLocation _ballcollision (Math|Vector|Lerp(Vector) (Transformation|GetActorLocation) (Transformation|GetActorLocation (Utilities|Array|Get(acopy) _outactors (stale EventBpiHandBallPass Zone_Index))) _floattrack_3) false false)
              (Physics|SetSimulatePhysics _ballcollision true)
              (Utilities|IsValid self
                (:Is%20Valid
                  (Physics|SetSimulatePhysics (Variables|Default|GetBallCollision) true)
                  (Utilities|IsValid self
                    (:Is%20Valid
                      (CallFunction|BallFinish)
                      (Actor|DestroyActor))))))))))))

(event EventBpiHandBallPass
  (params (Zone_Index :type Integer) (HandBallerPosition :type E_HandBallerCapturePosition%20Enum :default "NewEnumerator0") (X :type Float%20%28single-precision%29) (Y :type Float%20%28single-precision%29) (Ready? :type Boolean) (IsGoa\Out? :type Boolean) (Refand? :type Boolean) (e_BallStates :type E_BallStates%20Enum :default "NewEnumerator0") (E_HandBallerBodyPoints :type E_HandBallerBodyPoints%20Enum :default "NewEnumerator0") (e_GameEtap :type E_GameEtape%20Enum :default "NewEnumerator3") (Captured :type Boolean) (PointLocation :type Vector :default "0, 0, 0")))

(event EventTick
  (params (DeltaSeconds :type Float%20%28single-precision%29)))

(fn ConstructionScript)

(fn BallFinish
  (Development|PrintString "Finish" true true "(R=0.703649,G=0.091223,B=1.000000,A=1.000000)"))