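; BP_BallSpawner spawns balls for a handball test game.
; BeginPlay caches TargetPoints tagged "Start", and ProjectileBall spawns a BP_Ball_2 at the point indexed by zone.
; Ball calls ProjectileBall, then spawns a BP_Ball at the projectile arrow with randomly scaled rotation.
; Reset re-fires ProjectileBall and calls an empty Respawn, Rickoshet triggers Ricochet on the first BP_Ball found, and the goal/out event is a stub.
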(event Custom|ProjectileBall
  (params (ZoneIndex :type Integer))
  (Game|SpawnActorfromClass "/Game/HandBallTest/BP/BP_Ball_2.BP_Ball_2_C" (Math|Transform|MakeTransform (Transformation|GetActorLocation (Utilities|Array|Get(acopy) (Variables|Default|GetStartPontsRef) ZoneIndex)) "0, 0, 0" "1,1,1") "Undefined" 0 false 0))

(event Custom|Goal\Out
  (params (Goal\Out? :type Boolean)))

(event Custom|Respawn)

(event EventBeginPlay
  (bind _outactors (Actor|GetAllActorsOfClasswithTag "/Script/Engine.TargetPoint" "Start"))
  (Variables|Default|SetStartPontsRef _outactors))

(event Collision|EventActorBeginOverlap
  (params (OtherActor :type Actor%20Object%20Reference)))

(event EventTick
  (params (DeltaSeconds :type Float%20%28single-precision%29)))

(event EventBpiHandBallPass
  (params (Zone_Index :type Integer) (HandBallerPosition :type E_HandBallerCapturePosition%20Enum :default "NewEnumerator0") (X :type Float%20%28single-precision%29) (Y :type Float%20%28single-precision%29) (Ready? :type Boolean) (IsGoa\Out? :type Boolean) (Refand? :type Boolean) (e_BallStates :type E_BallStates%20Enum :default "NewEnumerator0") (E_HandBallerBodyPoints :type E_HandBallerBodyPoints%20Enum :default "NewEnumerator0") (e_GameEtap :type E_GameEtape%20Enum :default "NewEnumerator3") (Captured :type Boolean) (PointLocation :type Vector :default "0, 0, 0")))

(fn ConstructionScript)

(fn Ball
  (bind _arrowprojectile (Variables|Default|GetArrowProjectile))
  (bind _returnvalue (Transformation|GetWorldTransform _arrowprojectile))
  (CallFunction|ProjectileBall (Variables|Default|GetZoneIndex))
  (Game|SpawnActorfromClass "/Game/HandBallTest/BP/BP_Ball.BP_Ball_C" (Math|Transform|MakeTransform (.location _returnvalue) (Math|Rotator|MakeRotator (* (.roll (.rotation _returnvalue)) (Math|Random|RandomFloatinRange 5e+02 1e+03)) (* (.pitch (.rotation _returnvalue)) (Math|Random|RandomFloatinRange 5e+02 1e+03)) (* (.yaw (.rotation _returnvalue)) (Math|Random|RandomFloatinRange 5e+02 1e+03))) "1,1,1") "Undefined" 0 false 0))

(fn Rickoshet
  (bind _outactors (Actor|GetAllActorsOfClass "/Game/HandBallTest/BP/BP_Ball.BP_Ball_C"))
  (Utilities|Casting|CastToBP_Ball (Utilities|Array|Get(acopy) _outactors))
  (Default|Ricochet (Utilities|Array|Get(acopy) _outactors)))

(fn Reset
  (CallFunction|ProjectileBall (Variables|Default|GetZoneIndex))
  (CallFunction|Respawn))

(fn Goal\Out?
  (CallFunction|Goal\Out false))