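; Handball ball actor that, on BeginPlay, flies to the "Gate" TargetPoint chosen by ZoneIndex, whose Comp_handball decides the path.
; On IsGoalOut, it passes position data to PlayerCharacterHandBall_BP and timeline-lerps to that character's hand or foot socket.
; Otherwise it lerps to the target point.
; Both paths then enable physics, set the character's ReadyIdle and destroy the ball after delays; collision overlaps add a random impulse.
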(event OnComponentBeginOverlap(BallCollision)
  (params (OverlappedComponent :type Primitive%20Component%20Object%20Reference) (OtherActor :type Actor%20Object%20Reference) (OtherComp :type Primitive%20Component%20Object%20Reference) (OtherBodyIndex :type Integer) (bFromSweep :type Boolean) (SweepResult :type Hit%20Result%20Structure%20%28by%20ref%29))
  (Utilities|FlowControl|Delay 1.0)
  (Transformation|SetActorRotation (* (.rotation (Transformation|GetActorTransform)) (Math|Random|RandomFloat)))
  (Physics|SetSimulatePhysics (Variables|Default|GetBall1) true)
  (Physics|AddImpulse (Variables|Default|GetBall1) (Math|Vector|MakeVector (Math|Random|RandomFloat) (Math|Random|RandomFloat) (Math|Random|RandomFloat)) "None" false)
  (Utilities|FlowControl|Delay 5.0)
  (Actor|DestroyActor))

(event EventBeginPlay
  (bind _outactors (Actor|GetAllActorsOfClasswithTag "/Script/Engine.TargetPoint" "Gate"))
  (bind _outactors_2 (Actor|GetAllActorsOfClass "/Game/HandBallTest/BP/PlayerCharacterHandBall_BP.PlayerCharacterHandBall_BP_C"))
  (bind _asplayer_character_hand_ball_bp (Utilities|Casting|CastToPlayerCharacterHandBall_BP (Utilities|Array|Get(acopy) _outactors_2)))
  (if (Variables|/Game/HandBallTest/BP/comp_handball.comp_handball_C|GetIsGoal\Out? (Actor|GetComponentbyClass (Utilities|Array|Get(acopy) _outactors (stale EventBpiHandBallPass Zone_Index)) "/Game/HandBallTest/BP/comp_handball.comp_handball_C"))
    (Variables|/Game/HandBallTest/BP/PlayerCharacterHandBall_BP.PlayerCharacterHandBall_BP_C|SetXpos _asplayer_character_hand_ball_bp (Variables|/Game/HandBallTest/BP/comp_handball.comp_handball_C|Getpos_X (Actor|GetComponentbyClass (Utilities|Array|Get(acopy) _outactors (stale EventBpiHandBallPass Zone_Index)) "/Game/HandBallTest/BP/comp_handball.comp_handball_C")))
    (Variables|/Game/HandBallTest/BP/PlayerCharacterHandBall_BP.PlayerCharacterHandBall_BP_C|SetYpos _asplayer_character_hand_ball_bp (Variables|/Game/HandBallTest/BP/comp_handball.comp_handball_C|Getpos_Y (Actor|GetComponentbyClass (Utilities|Array|Get(acopy) _outactors (stale EventBpiHandBallPass Zone_Index)) "/Game/HandBallTest/BP/comp_handball.comp_handball_C")))
    (Variables|/Game/HandBallTest/BP/PlayerCharacterHandBall_BP.PlayerCharacterHandBall_BP_C|SetGoal\Out? _asplayer_character_hand_ball_bp (Variables|/Game/HandBallTest/BP/comp_handball.comp_handball_C|GetIsGoal\Out? (Actor|GetComponentbyClass (Utilities|Array|Get(acopy) _outactors (stale EventBpiHandBallPass Zone_Index)) "/Game/HandBallTest/BP/comp_handball.comp_handball_C")))
    (switch Utilities|FlowControl|Switch|SwitchonE_HandBallerBodyPoints (Variables|/Game/HandBallTest/BP/comp_handball.comp_handball_C|GetE_HandBallerBodyPoints (Actor|GetComponentbyClass (Utilities|Array|Get(acopy) _outactors (stale EventBpiHandBallPass Zone_Index)) "/Game/HandBallTest/BP/comp_handball.comp_handball_C"))
      (:NewEnumerator0
        (Variables|Default|Setsocketindex 0)
        (bind _floattrack (Timeline|Timeline_4 Play)
          (:Update
            (Transformation|SetActorLocation (Math|Vector|Lerp(Vector) (Transformation|GetActorLocation) (Transformation|GetSocketLocation (Variables|/Script/Engine.Character|GetMesh _asplayer_character_hand_ball_bp) (Utilities|Array|Get(acopy) (Variables|/Game/HandBallTest/BP/PlayerCharacterHandBall_BP.PlayerCharacterHandBall_BP_C|GetIn%20Socket%20Name _asplayer_character_hand_ball_bp) (Variables|Default|Getsocketindex))) _floattrack) false false)
            (Utilities|FlowControl|Delay 0.2)
            (Transformation|SetActorRotation (* (.rotation (Transformation|GetActorTransform)) (Math|Random|RandomFloat)))
            (Physics|SetSimulatePhysics (Variables|Default|GetBall1) true)
            (Utilities|FlowControl|Delay 2.0)
            (Variables|/Game/HandBallTest/BP/PlayerCharacterHandBall_BP.PlayerCharacterHandBall_BP_C|SetReady/Idle? _asplayer_character_hand_ball_bp true)
            (Utilities|FlowControl|Delay 5.0)
            (Actor|DestroyActor))))
      (:NewEnumerator1
        (Variables|Default|Setsocketindex 1)
        (Timeline|Timeline_4 Play))
      (:NewEnumerator2
        (Variables|Default|Setsocketindex 2)
        (Timeline|Timeline_4 Play))
      (:NewEnumerator3
        (Variables|Default|Setsocketindex 3)
        (Timeline|Timeline_4 Play)))
    (else
      (bind _floattrack_2 (Timeline|Timeline_0 Play)
        (:Update
          (Transformation|SetWorldLocation (Variables|Default|GetBall1) (Math|Vector|Lerp(Vector) (Transformation|GetActorLocation) (Transformation|GetActorLocation (Utilities|Array|Get(acopy) _outactors (stale EventBpiHandBallPass Zone_Index))) _floattrack_2) false false)
          (Utilities|FlowControl|Delay 0.1)
          (Transformation|SetActorRotation (* (.rotation (Transformation|GetActorTransform)) (Math|Random|RandomFloat)))
          (Physics|SetSimulatePhysics (Variables|Default|GetBall1) true)
          (Variables|/Game/HandBallTest/BP/PlayerCharacterHandBall_BP.PlayerCharacterHandBall_BP_C|SetReady/Idle? _asplayer_character_hand_ball_bp true)
          (Utilities|FlowControl|Delay 5.0)
          (Actor|DestroyActor))))))

(event Collision|EventActorBeginOverlap
  (params (OtherActor :type Actor%20Object%20Reference)))

(event EventBpiHandBallPass
  (params (Zone_Index :type Integer) (HandBallerPosition :type E_HandBallerCapturePosition%20Enum :default "NewEnumerator0") (X :type Float%20%28single-precision%29) (Y :type Float%20%28single-precision%29) (Ready? :type Boolean) (IsGoa\Out? :type Boolean) (Refand? :type Boolean) (e_BallStates :type E_BallStates%20Enum :default "NewEnumerator0") (E_HandBallerBodyPoints :type E_HandBallerBodyPoints%20Enum :default "NewEnumerator0") (e_GameEtap :type E_GameEtape%20Enum :default "NewEnumerator3") (Captured :type Boolean)))

(event EventTick
  (params (DeltaSeconds :type Float%20%28single-precision%29)))

(fn ConstructionScript)