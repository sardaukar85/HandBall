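; Handball test ball actor that flies to a "Gate"-tagged TargetPoint, then destroys itself.
; BeginPlay and the BpiHandBallPass event share one path: disable physics, briefly wait, then play a timeline that lerps Ball1 toward the target picked by ZoneIndex.
; Each timeline update also randomly scales the actor's rotation, re-enables physics and reaches a delayed DestroyActor.
; Hit and overlap events are empty, and several leftover impulse, attach and destroy chains are unconnected.
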(event OnComponentBeginOverlap(Ball1)
  (params (OverlappedComponent :type Primitive%20Component%20Object%20Reference) (OtherActor :type Actor%20Object%20Reference) (OtherComp :type Primitive%20Component%20Object%20Reference) (OtherBodyIndex :type Integer) (bFromSweep :type Boolean) (SweepResult :type Hit%20Result%20Structure%20%28by%20ref%29)))

(event OnComponentHit(Ball1)
  (params (HitComponent :type Primitive%20Component%20Object%20Reference) (OtherActor :type Actor%20Object%20Reference) (OtherComp :type Primitive%20Component%20Object%20Reference) (NormalImpulse :type Vector :default "0, 0, 0") (Hit :type Hit%20Result%20Structure%20%28by%20ref%29)))

(event Custom|CustomEvent_0)

(event EventBeginPlay
  (Physics|SetSimulatePhysics (Variables|Default|GetBall1) false)
  (Utilities|FlowControl|Delay 0.1)
  (bind _outactors (Actor|GetAllActorsOfClasswithTag "/Script/Engine.TargetPoint" "Gate"))
  (bind _floattrack (Timeline|Timeline_0 Play)
    (:Update
      (Transformation|SetWorldLocation (Variables|Default|GetBall1) (Math|Vector|Lerp(Vector) (Transformation|GetActorLocation) (Transformation|GetActorLocation (Utilities|Array|Get(acopy) _outactors (stale EventBpiHandBallPass Zone_Index))) _floattrack) false false)
      (Transformation|SetActorRotation (* (.rotation (Transformation|GetActorTransform)) (Math|Random|RandomFloat)))
      (Physics|SetSimulatePhysics (Variables|Default|GetBall1) true)
      (Utilities|FlowControl|Delay 6.0)
      (Actor|DestroyActor))))

(event Collision|EventActorBeginOverlap
  (params (OtherActor :type Actor%20Object%20Reference)))

(event EventBpiHandBallPass
  (params (Zone_Index :type Integer) (HandBallerPosition :type E_HandBallerCapturePosition%20Enum :default "NewEnumerator0") (X :type Float%20%28single-precision%29) (Y :type Float%20%28single-precision%29) (Ready? :type Boolean) (IsGoa\Out? :type Boolean) (Refand? :type Boolean) (e_BallStates :type E_BallStates%20Enum :default "NewEnumerator0") (E_HandBallerBodyPoints :type E_HandBallerBodyPoints%20Enum :default "NewEnumerator0") (e_GameEtap :type E_GameEtape%20Enum :default "NewEnumerator3") (Captured :type Boolean))
  (Physics|SetSimulatePhysics (Variables|Default|GetBall1) false)
  (Utilities|FlowControl|Delay 0.1)
  (bind _outactors (Actor|GetAllActorsOfClasswithTag "/Script/Engine.TargetPoint" "Gate"))
  (bind _floattrack (Timeline|Timeline_0 Play)
    (:Update
      (Transformation|SetWorldLocation (Variables|Default|GetBall1) (Math|Vector|Lerp(Vector) (Transformation|GetActorLocation) (Transformation|GetActorLocation (Utilities|Array|Get(acopy) _outactors Zone_Index)) _floattrack) false false)
      (Transformation|SetActorRotation (* (.rotation (Transformation|GetActorTransform)) (Math|Random|RandomFloat)))
      (Physics|SetSimulatePhysics (Variables|Default|GetBall1) true)
      (Utilities|FlowControl|Delay 6.0)
      (Actor|DestroyActor))))

(event EventTick
  (params (DeltaSeconds :type Float%20%28single-precision%29)))

(fn ConstructionScript)