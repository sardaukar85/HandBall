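; BP_EmissiveMarker is a marker actor in the hand-ball test whose four planes are shown or hidden together.
; VisibleOn shows the planes through a FlipFlop with only A wired, so it acts on alternate calls, while VisibleOff hides them.
; Both record the state in IsVisible.
; The game-stage event is empty, and disconnected logic would show the planes only during Ready for Capture.
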(event Custom|CustomEvent_0)

(event Collision|EventActorBeginOverlap
  (params (OtherActor :type Actor%20Object%20Reference)))

(event EventTick
  (params (DeltaSeconds :type Float%20%28single-precision%29)))

(event EventBpiHandBallPass
  (params (Zone_Index :type Integer) (GameState :type E_GameEtape%20Enum :default "NewEnumerator3") (HandBallerPosition :type E_HandBallerCapturePosition%20Enum :default "NewEnumerator0") (X :type Float%20%28single-precision%29) (Y :type Float%20%28single-precision%29) (Ready? :type Boolean) (IsGoa\Out? :type Boolean) (Refand? :type Boolean) (e_BallStates :type E_BallStates%20Enum :default "NewEnumerator0") (E_HandBallerBodyPoints :type E_HandBallerBodyPoints%20Enum :default "NewEnumerator0") (e_GameEtap :type E_GameEtape%20Enum :default "NewEnumerator3")))

(event EventBeginPlay)

(fn ConstructionScript)

(fn 1Visibleon
  (Utilities|FlowControl|FlipFlop
    (:A
      (bind _output_get (Variables|Default|SetIsVisible? true))
      (Rendering|SetVisibility (Variables|Default|GetPlane1) _output_get false))))

(fn 2VisibleOff
  (bind _output_get (Variables|Default|SetIsVisible? false))
  (Rendering|SetVisibility (Variables|Default|GetPlane1) _output_get false))