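; BP_FX_Emiter is an effect actor in the HandBallTest game that briefly shows a Niagara effect in response to a handball pass event.
; The Niagara component is hidden on BeginPlay.
; BpiHandBallPass sets its visibility from the IsGoaOut flag, ignoring GameState, then hides it again after a short delay.
; The FXStart event is empty, and the older ParticleSystem and GameState-switch logic is left disconnected.
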(event Custom|FXStart)

(event EventBeginPlay
  (Rendering|SetVisibility (Variables|Default|GetNiagara) false false))

(event Collision|EventActorBeginOverlap
  (params (OtherActor :type Actor%20Object%20Reference)))

(event EventTick
  (params (DeltaSeconds :type Float%20%28single-precision%29)))

(event EventBpiHandBallPass
  (params (Zone_Index :type Integer) (GameState :type E_GameEtape%20Enum :default "NewEnumerator3") (IsGoa\Out? :type Boolean) (HandBallerPosition :type E_HandBallerCapturePosition%20Enum :default "NewEnumerator0") (X :type Float%20%28single-precision%29) (Y :type Float%20%28single-precision%29))
  (bind _niagara (Variables|Default|GetNiagara))
  (Rendering|SetVisibility _niagara IsGoa\Out? false)
  (Utilities|FlowControl|Delay 3.0)
  (Rendering|SetVisibility _niagara false false))

(fn ConstructionScript)