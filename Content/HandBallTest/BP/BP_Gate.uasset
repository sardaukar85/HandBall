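; BP_Gate is the gate actor in a handball test that removes the ball and displays a zone number.
; Any begin overlap on GateCollision destroys the referenced BP_Ball, then casts the manager reference with no further action, as the IsReadyForCapture write is disconnected.
; The BpiHandBallPass event receives a zone index and shows it one-based on the IndexBall text.
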(event OnComponentHit(GateCollision)
  (params (HitComponent :type Primitive%20Component%20Object%20Reference) (OtherActor :type Actor%20Object%20Reference) (OtherComp :type Primitive%20Component%20Object%20Reference) (NormalImpulse :type Vector :default "0, 0, 0") (Hit :type Hit%20Result%20Structure%20%28by%20ref%29)))

(event OnComponentBeginOverlap(GateCollision)
  (params (OverlappedComponent :type Primitive%20Component%20Object%20Reference) (OtherActor :type Actor%20Object%20Reference) (OtherComp :type Primitive%20Component%20Object%20Reference) (OtherBodyIndex :type Integer) (bFromSweep :type Boolean) (SweepResult :type Hit%20Result%20Structure%20%28by%20ref%29))
  (bind _ballref (Variables|Default|GetBallRef))
  (Utilities|FlowControl|Sequence
    (:then_0
      (Utilities|Casting|CastToBP_Ball _ballref)
      (Actor|DestroyActor _ballref))
    (:then_1
      (bind _asbp_hand_ball_manager (Utilities|Casting|CastToBP_HandBall_Manager (Variables|Default|GetHandBallManagerRef))))))

(event EventBeginPlay)

(event Collision|EventActorBeginOverlap
  (params (OtherActor :type Actor%20Object%20Reference)))

(event EventTick
  (params (DeltaSeconds :type Float%20%28single-precision%29)))

(event EventBpiHandBallPass
  (params (Zone_Index :type Integer) (HandBallerPosition :type E_HandBallerCapturePosition%20Enum :default "NewEnumerator0") (X :type Float%20%28single-precision%29) (Y :type Float%20%28single-precision%29) (Ready? :type Boolean) (IsGoa\Out? :type Boolean) (Refand? :type Boolean) (e_BallStates :type E_BallStates%20Enum :default "NewEnumerator0") (E_HandBallerBodyPoints :type E_HandBallerBodyPoints%20Enum :default "NewEnumerator0") (e_GameEtap :type E_GameEtape%20Enum :default "NewEnumerator3") (Captured :type Boolean) (PointLocation :type Vector :default "0, 0, 0"))
  (Rendering|Components|TextRender|SetText (Variables|Default|GetIndexBall) (Utilities|Text|ToText(Integer) (+ Zone_Index 1))))

(fn ConstructionScript)