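; Blueprint sound source for the handball test that plays 2D audio cues for each game stage.
; The BpiHandBallPass interface event maps the EGameEtap stage to an index in a Sound array, choosing a goal or out cue at the Result stage from IsGoaOut.
; Separate Prepare, Goal, Out and Stop functions play fixed entries directly, while Ready and Result functions are empty.
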(event EventBeginPlay)

(event EventBpiHandBallPass
  (params (Zone_Index :type Integer) (GameState :type E_GameEtape%20Enum :default "NewEnumerator3") (HandBallerPosition :type E_HandBallerCapturePosition%20Enum :default "NewEnumerator0") (X :type Float%20%28single-precision%29) (Y :type Float%20%28single-precision%29) (Ready? :type Boolean) (IsGoa\Out? :type Boolean) (Refand? :type Boolean) (e_BallStates :type E_BallStates%20Enum :default "NewEnumerator0") (E_HandBallerBodyPoints :type E_HandBallerBodyPoints%20Enum :default "NewEnumerator0") (e_GameEtap :type E_GameEtape%20Enum :default "NewEnumerator3"))
  (switch Utilities|FlowControl|Switch|SwitchonE_GameEtape e_GameEtap
    (:NewEnumerator3
      (Variables|Default|SetSoundIndex 0))
    (:NewEnumerator0
      (Variables|Default|SetSoundIndex 1))
    (:NewEnumerator1
      (Variables|Default|SetSoundIndex 2))
    (:NewEnumerator2
      (if IsGoa\Out?
        (Variables|Default|SetSoundIndex 3)
        (else
          (Variables|Default|SetSoundIndex 4)))))
  (Audio|PlaySound2D (Utilities|Array|Get(acopy) (Variables|Default|GetSound) (Variables|Default|GetSoundIndex)) 1.0 1.0 0.0 0 0))

(fn ConstructionScript)

(fn 1Prepare
  (bind _output_get (Variables|Default|SetSoundIndex 0))
  (Audio|PlaySound2D (Utilities|Array|Get(acopy) (Variables|Default|GetSound) _output_get) 1.0 1.0 0.0 0 0))

(fn 2Ready)

(fn 3Goal
  (bind _output_get (Variables|Default|SetSoundIndex 3))
  (Audio|PlaySound2D (Utilities|Array|Get(acopy) (Variables|Default|GetSound) _output_get) 1.0 1.0 0.0 0 0))

(fn 3Out
  (bind _output_get (Variables|Default|SetSoundIndex 4))
  (Audio|PlaySound2D (Utilities|Array|Get(acopy) (Variables|Default|GetSound) _output_get) 1.0 1.0 0.0 0 0))

(fn 4Result)

(fn 0Stop
  (Audio|PlaySound2D (Utilities|Array|Get(acopy) (Variables|Default|GetSound)) 1.0 1.0 0.0 0 0))