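; BP_HandBall_Manager is a handball test manager that is currently mostly a stub.
; Its live logic only prints debug strings when the BPI_HandBall pass event fires or the Spawn input is pressed, while BeginPlay leads nowhere.
; Disconnected nodes hold unused logic for launching balls from BP_BallSpawner, updating BP_Text by goal-out result, and setting game state and zone index.
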(event EventBeginPlay
  (Utilities|FlowControl|Sequence))

(event Collision|EventActorBeginOverlap
  (params (OtherActor :type Actor%20Object%20Reference)))

(event EventTick
  (params (DeltaSeconds :type Float%20%28single-precision%29)))

(event EventBpiHandBallPass
  (params (Zone_Index :type Integer) (GameState :type E_GameEtape%20Enum :default "NewEnumerator3") (IsGoa\Out? :type Boolean) (HandBallerPosition :type E_HandBallerCapturePosition%20Enum :default "NewEnumerator0") (X :type Float%20%28single-precision%29) (Y :type Float%20%28single-precision%29) (Ready? :type Boolean) (Captured\Refand? :type Boolean) (e_BallStates :type E_BallStates%20Enum :default "NewEnumerator0"))
  (Utilities|FlowControl|Sequence
    (:then_0
      (Development|PrintString "Manager" true true "(R=0.000000,G=1.000000,B=0.668012,A=1.000000)"))))

(event Input|ActionEvents|InputActionSpawn
  (params (Key :type Key%20Structure))
  (:Pressed
    (Development|PrintString "Spawn")))

(fn ConstructionScript)