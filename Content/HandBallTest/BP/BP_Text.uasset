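; BP_Text is a HandBallTest actor that displays status messages on a Text3D component, picked by index from a TXTNames array.
; The construction script sets one entry as the initial text, and BeginPlay switches it to another.
; The BpiHandBallPass event switches on EGameEtap with no cases wired.
; A disconnected, never-run chain would show a Ready-dependent message after a delay, then restore the initial text.
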(event EventBeginPlay
  (Class|Text3DComponent|SetText (Variables|Default|GetText3D) (Utilities|Array|Get(acopy) (Variables|Default|GetTXT_Names) 2)))

(event Collision|EventActorBeginOverlap
  (params (OtherActor :type Actor%20Object%20Reference)))

(event EventTick
  (params (DeltaSeconds :type Float%20%28single-precision%29)))

(event EventBpiHandBallPass
  (params (Zone_Index :type Integer) (GameState :type E_GameEtape%20Enum :default "NewEnumerator3") (HandBallerPosition :type E_HandBallerCapturePosition%20Enum :default "NewEnumerator0") (X :type Float%20%28single-precision%29) (Y :type Float%20%28single-precision%29) (Ready? :type Boolean) (IsGoa\Out? :type Boolean) (Refand? :type Boolean) (e_BallStates :type E_BallStates%20Enum :default "NewEnumerator0") (E_HandBallerBodyPoints :type E_HandBallerBodyPoints%20Enum :default "NewEnumerator0") (e_GameEtap :type E_GameEtape%20Enum :default "NewEnumerator3"))
  (switch Utilities|FlowControl|Switch|SwitchonE_GameEtape e_GameEtap))

(fn ConstructionScript
  (Class|Text3DComponent|SetText (Variables|Default|GetText3D) (Utilities|Array|Get(acopy) (Variables|Default|GetTXT_Names) 1)))