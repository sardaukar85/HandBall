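; Player character for a handball test that can hold and release the ball.
; Capture attaches the first BP_Ball found in the level to the mesh's right-hand socket, and Detach releases it in world space.
; BpiHandBallPass copies incoming position, readiness, goal-out, captured and ball-state values into variables.
; MoveTo, goal, out and capsule overlap events are empty, and some older capture logic is left unconnected.
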(event OnComponentBeginOverlap(CapsuleComponent)
  (params (OverlappedComponent :type Primitive%20Component%20Object%20Reference) (OtherActor :type Actor%20Object%20Reference) (OtherComp :type Primitive%20Component%20Object%20Reference) (OtherBodyIndex :type Integer) (bFromSweep :type Boolean) (SweepResult :type Hit%20Result%20Structure%20%28by%20ref%29)))

(event Custom|Capture
  (bind _outactors (Actor|GetAllActorsOfClass "/Game/HandBallTest/BP/BP_Ball.BP_Ball_C"))
  (Transformation|AttachComponentToComponent (Utilities|Array|Get(acopy) _outactors) (Variables|Character|GetMesh) "RightHandSocket" "KeepRelative" "KeepRelative" "KeepRelative" true))

(event Custom|MoveTo
  (params (PointIndex :type Integer)))

(event Custom|Out!)

(event Custom|Goal!)

(event Custom|Detach
  (bind _outactors (Actor|GetAllActorsOfClass "/Game/HandBallTest/BP/BP_Ball.BP_Ball_C"))
  (Transformation|DetachFromActor (Utilities|Array|Get(acopy) _outactors) "KeepWorld" "KeepWorld" "KeepWorld"))

(event EventBeginPlay)

(event Collision|EventActorBeginOverlap
  (params (OtherActor :type Actor%20Object%20Reference)))

(event EventTick
  (params (DeltaSeconds :type Float%20%28single-precision%29)))

(event EventBpiHandBallPass
  (params (Zone_Index :type Integer) (GameState :type E_GameEtape%20Enum :default "NewEnumerator3") (IsGoa\Out? :type Boolean) (HandBallerPosition :type E_HandBallerCapturePosition%20Enum :default "NewEnumerator0") (X :type Float%20%28single-precision%29) (Y :type Float%20%28single-precision%29) (Ready? :type Boolean) (Captured\Refand? :type Boolean) (e_BallStates :type E_BallStates%20Enum :default "NewEnumerator0"))
  (Utilities|FlowControl|Sequence
    (:then_1
      (Variables|Default|SetXpos X)
      (Variables|Default|SetYpos Y)
      (Variables|Default|SetReady? Ready?)
      (Variables|Default|SetGoal\Out? IsGoa\Out?)
      (Variables|Default|SetCaptured\Refand? Captured\Refand?)
      (Variables|Default|Sete_BallState e_BallStates))))

(fn ConstructionScript)